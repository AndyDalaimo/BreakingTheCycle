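; BP_BorisLightDistraction is a world-interaction distraction that makes a light flicker when the player triggers it.
; On the player-triggered state, a Timeline restarts and its Flicker Rate event track drives a FlipFlop that toggles the LightDistraction component's visibility.
; On the resolved state, it prints a debug message, stops the Timeline and leaves the light visible.
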(event `self.PlayerTriggeredEventState`
  (bind _lightdistraction (`self.LightDistraction`))
  ;[1 1 1] Triggered on State change. Aesthetic changes here
  (`Timeline|Timeline` :!via `PlayFromStart`
    (:`FlickerRate`
      (`/Engine/EditorBlueprintResources/StandardMacros.FlipFlop`
        (:`A`
          (`SceneComponent.SetVisibility` _lightdistraction true false))
        (:`B`
          (`SceneComponent.SetVisibility` _lightdistraction false false))))))

(event `self.ResolvedEventState`
  ;[1 1 1] Triggered on State change. Aesthetic changes here
  (`KismetSystemLibrary.PrintString` "Resolved")
  (`TimelineComponent.Stop` (`self.Timeline`))
  (`SceneComponent.SetVisibility` (`self.LightDistraction`) true false))

(fn `UserConstructionScript`)