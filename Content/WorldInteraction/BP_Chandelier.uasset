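; BP_Chandelier is the world interaction object that can kill the Nobleman and end the game.
; Singer interactions increment AliceInteractCounter; a Nobleman interaction triggers the death if the end sequence is flagged and the counter exceeds one.
; The death plays a level sequence, marks the Nobleman DEAD in HouseStateMachine and zeroes all HouseCharacters' walk speed.
; After a delay, it stops the sequence and shows the WB_End widget.
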(event `self.ReceiveBeginPlay`
  (bind _returnvalue (`GameplayStatics.GetActorOfClass` "/Script/BreakingTheCycle.HouseStateMachine"))
  (set `self.StateMachineRef` _returnvalue)
  (bind _outactors (`GameplayStatics.GetAllActorsOfClass` "/Script/BreakingTheCycle.HouseCharacter"))
  (set `self.HouseCharacters` _outactors))

(event `self.CharacterInteractionEvent`
  (params (name :type "ECharacterName Enum" :default "NONE") (actor :type "HouseCharacter Object Reference"))
  ;[1 1 1] event called on Character Overlap.
  ; If End sequence is triggered, the Nobleman will die by the Chandelier
  (switch `ECharacterName` name
    (:`NOBLEMAN`
      (if (and (`self.bEndSequenceTriggered`) (> (`self.AliceInteractCounter`) 1))
        (`KismetSystemLibrary.PrintString` "end for the nobleman")
        (`WidgetLayoutLibrary.RemoveAllWidgets`)
        (bind _outactor (`LevelSequencePlayer.CreateLevelSequencePlayer` (`self.sequence`) (make `MovieSceneSequencePlaybackSettings` false (make `MovieSceneSequenceLoopCount` 0))))
        (bind _sequenceplayer (`LevelSequenceActor.SequencePlayer` _outactor))
        (`MovieSceneSequencePlayer.Play` _sequenceplayer)
        (`HouseStateMachine.ChangeCharacterState` (`self.StateMachineRef`) (make `CurrentState` "NOBLEMAN"))
        (for _array_element (`self.HouseCharacters`)
          (set `CharacterMovementComponent.MaxWalkSpeed` 0.0 (`Character.CharacterMovement` _array_element)))
        (`KismetSystemLibrary.Delay` 7.0)
        (`MovieSceneSequencePlayer.Stop` _sequenceplayer)
        (bind _returnvalue (`|CreateWidget` "/Game/EmStuff/UI/Widgets/WB_End.WB_End_C" (`GameplayStatics.GetPlayerController` 0)))
        (`UserWidget.AddToViewport` _returnvalue 0)
        (else
          (`KismetSystemLibrary.PrintString` "He lives another day"))))
    (:`SINGER`
      (bind _output_get (set `self.AliceInteractCounter` (+ (`self.AliceInteractCounter`) 1)))
      (`KismetSystemLibrary.PrintString` (`KismetStringLibrary.Conv_ByteToString` _output_get)))))

(fn `UserConstructionScript`)